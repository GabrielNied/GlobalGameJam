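; WillyController is a controller Blueprint that handles pausing the game.
; On BeginPlay it creates a PauseMenu widget once and stores it for reuse.
; The Pause input action toggles the game's paused state, adding the menu to the player screen and showing the mouse cursor, or removing both on resume.
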(event EventBeginPlay
  (bind _returnvalue (UserInterface|CreateWidget "/Game/Blueprints/UI/Game/PauseMenu.PauseMenu_C"))
  (Variables|Default|SetPauseMenu _returnvalue))

(event Input|ActionEvents|InputActionPause
  (params (Key :type Key%20Structure :default "None"))
  (bind _pausemenu (Variables|Default|GetPauseMenu))
  (:Pressed
    (if (Game|IsGamePaused)
      (Game|SetGamePaused false)
      (Widget|RemovefromParent _pausemenu)
      (Variables|Default|SetbShowMouseCursor false)
      (else
        (Game|SetGamePaused true)
        (UserInterface|Viewport|AddtoPlayerScreen _pausemenu)
        (Variables|Default|SetbShowMouseCursor true)))))

(fn ConstructionScript)