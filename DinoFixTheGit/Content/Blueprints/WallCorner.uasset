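; WallCorner is a repairable wall corner piece that a PaperPlayer restores while overlapping its collision.
; Repair takes the first overlapping player and, while that player is repairing, re-schedules itself on a one-second timer and adds clamped WallLife.
; At full life it clears the broken flag and re-enables player movement.
; An IsBroken check is left unconnected, so repair does not depend on it.
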(fn ConstructionScript)

(fn Repair
  (bind _aspaper_player (Utilities|Casting|CastToPaperPlayer (Utilities|Array|Get(acopy) (Collision|GetOverlappingActors (Variables|Default|GetCollision) "/Game/Blueprints/PaperPlayer.PaperPlayer_C" :!class /Script/Engine.PrimitiveComponent))))
  (if (Variables|/Game/Blueprints/PaperPlayer.PaperPlayer_C|GetIsRepairing _aspaper_player)
    (Utilities|Time|SetTimerbyFunctionName 0 "Repair" 1.0)
    (bind _output_get (Variables|Default|SetWallLife (Math|Float|Clamp(Float) (+ (Variables|Default|GetWallLife) 5.0) 0.0 1e+02)))
    (if (>= _output_get 1e+02)
      (Variables|Default|SetIsBroken false)
      (Variables|/Game/Blueprints/PaperPlayer.PaperPlayer_C|SetCanMove _aspaper_player true))))