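; WallNormal is a repairable wall that an overlapping PaperPlayer restores over time.
; Repair re-arms itself on a one-second timer while the player is repairing, adding a clamped increment to WallLife each pass and updating the player's progress bar widget.
; At full life it clears IsBroken, re-enables player movement and hides the bar.
; An IsBroken check is left disconnected.
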(fn ConstructionScript)

(fn Repair
  (bind _aspaper_player (Utilities|Casting|CastToPaperPlayer (Utilities|Array|Get(acopy) (Collision|GetOverlappingActors (Variables|Default|GetCollision) "/Game/Blueprints/PaperPlayer.PaperPlayer_C" :!class /Script/Engine.PrimitiveComponent))))
  (if (Variables|/Game/Blueprints/PaperPlayer.PaperPlayer_C|GetIsRepairing _aspaper_player)
    (Utilities|Time|SetTimerbyFunctionName 0 "Repair" 1.0)
    (bind _output_get (Variables|Default|SetWallLife (Math|Float|Clamp(Float) (+ (Variables|Default|GetWallLife) 0.05))))
    (bind _asprogress_bar_repair_bp (Utilities|Casting|CastToProgressBarRepairBP (UserInterface|GetUserWidgetObject (Variables|/Game/Blueprints/PaperPlayer.PaperPlayer_C|GetProgressBarRepairWidget _aspaper_player))))
    (Default|UpdateRepairBar _asprogress_bar_repair_bp _output_get)
    (if (>= _output_get 1.0)
      (Variables|Default|SetIsBroken false)
      (Variables|/Game/Blueprints/PaperPlayer.PaperPlayer_C|SetCanMove _aspaper_player true)
      (Rendering|SetVisibility (Variables|/Game/Blueprints/PaperPlayer.PaperPlayer_C|GetProgressBarRepairWidget _aspaper_player) false false))))