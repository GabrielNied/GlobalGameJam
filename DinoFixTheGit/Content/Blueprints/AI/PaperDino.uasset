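; PaperDino is an AI dinosaur pawn with pet-style needs that can post chores to the game's task widget.
; Looping timers drain hunger and sleep, while self-rescheduling functions refill them; eating builds toward pooping, which lowers hygiene.
; SetHumor averages hunger, hygiene and sleep for the humor bar and prompts DinoController to seek tasks.
; Seeing the player triggers following, wall overlaps are passed to the controller, and the fury timer is unwired.
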(event OnComponentBeginOverlap(CapsuleComponent)
  (params (OverlappedComponent :type Primitive%20Component%20Object%20Reference) (OtherActor :type Actor%20Object%20Reference) (OtherComp :type Primitive%20Component%20Object%20Reference) (OtherBodyIndex :type Integer) (bFromSweep :type Boolean) (SweepResult :type Hit%20Result%20Structure%20%28by%20ref%29))
  (if (Actor|ActorHasTag OtherActor "Wall")
    (bind _aswall_corner (Utilities|Casting|CastToWallCorner OtherActor))
    (Default|GetWall (Variables|Default|GetDinoController) _aswall_corner)))

(event OnSeePawn(PawnSensing)
  (params (Pawn :type Pawn%20Object%20Reference))
  (bind _dinocontroller (Variables|Default|GetDinoController))
  ;[1 1 1] Check LOS to player
  (bind _output_get (Variables|Default|SethasLOSofPlayer true))
  (if _output_get
    (Variables|Default|SetisBusy true)
    (Default|FollowPlayer _dinocontroller)
    (Utilities|FlowControl|RetriggerableDelay 1.0)
    (bind _output_get_2 (Variables|Default|SethasLOSofPlayer false))
    (if (not _output_get_2)
      (AI|Navigation|StopMovement _dinocontroller)
      ;[1 1 1] Back to Patrol
      (CallFunction|FinishedTask))))

(event Custom|FinishedTask
  (params (Task :type Text))
  ;[1 1 1] On finished task
  (if (Utilities|Enum|Equal(Enum) Task (Class|KismetTextLibrary|GetEmptyText))
    _
    (else
      (bind _asin_game (Utilities|Casting|CastToInGame (Game|GetGameMode)))
      (Default|SetTaskText (Variables|/Game/Blueprints/Gameloop/InGame.InGame_C|GetTasksWidget _asin_game) Task)
      (Development|PrintString "Hello")))
  (Utilities|FlowControl|Delay 2.0)
  (Variables|Default|SetisBusy false)
  (Development|PrintString "Terminou")
  (Default|SeekNewTask (Variables|Default|GetDinoController)))

(event EventBeginPlay
  ;[1 1 1] Start Dino
  ;[1 1 1] Deactivate enemy rotation
  (Variables|Default|SetbUseControllerRotationYaw false)
  ;[1 1 1] Set Dino Controller
  (bind _asdino_controller (Utilities|Casting|CastToDinoController (Pawn|GetController)))
  (Variables|Default|SetDinoController _asdino_controller)
  ;[1 1 1] Start loops
  (CallFunction|SetHumor)
  (Utilities|FlowControl|Delay 0.0)
  (Utilities|Time|SetTimerbyFunctionName 0 "FeelHungry" 5.0 true)
  (Utilities|Time|SetTimerbyFunctionName 0 "FeelSleep" 1e+01 true)
  (Utilities|FlowControl|Delay 5.0)
  (Variables|Default|SetisNeedToBreak true))

(fn ConstructionScript)

(fn FeelHungry
  (if (Variables|Default|GetisEating)
    (Development|PrintString "esperando terminar comida")
    (else
      (bind _output_get (Variables|Default|SethungryLevel (Math|Float|Clamp(Float) (- (Variables|Default|GethungryLevel) (Variables|Default|GethungerCoeficient)) 0.0 1e+02)))
      (if (<= _output_get (Variables|Default|GethungerBaseLevel))
        (Variables|Default|SetisHungry true))
      (Development|PrintString (Utilities|String|Append "Hungry: " (Utilities|String|ToString(Float) _output_get)) true true "(R=1.000000,G=0.604231,B=0.000000,A=1.000000)" 3.0)
      (CallFunction|SetHumor))))

(fn FeelFury
  (bind _output_get (Variables|Default|SetfuryLevel (Math|Float|Clamp(Float) (+ (Variables|Default|GetfuryLevel) (Variables|Default|GetfuryCoeficient)) 0.0 1e+02)))
  (CallFunction|SetHumor))

(fn ManageHygiene
  (bind _output_get (Variables|Default|SethygieneLevel (Math|Float|Clamp(Float) (- (Variables|Default|GethygieneLevel) (Variables|Default|GethygieneCoeficient)) 0.0 1e+02)))
  (CallFunction|SetHumor))

(fn FeelSleep
  (if (Variables|Default|GetisSleeping)
    (Development|PrintString "esperando terminar dormida")
    (else
      (bind _output_get (Variables|Default|SetsleepLevel (Math|Float|Clamp(Float) (- (Variables|Default|GetsleepLevel) (Variables|Default|GetsleepCoeficient)) 0.0 1e+02)))
      (if (<= _output_get (Variables|Default|GetsleepBaseLevel))
        (Variables|Default|SetisNeedToSleep true))
      (CallFunction|SetHumor)
      (Development|PrintString (Utilities|String|Append "Sleep: " (Utilities|String|ToString(Float) _output_get)) true true "(R=0.000000,G=1.000000,B=0.722583,A=1.000000)" 3.0))))

(fn Shit
  (bind _returnvalue (Transformation|GetActorTransform))
  (bind (_location _rotation _scale) (Math|Transform|BreakTransform _returnvalue))
  (bind (_x _y) (Math|Vector|BreakVector _location))
  (Development|PrintString "vai cagar")
  (Variables|Default|SethygieneLevel (Math|Float|Clamp(Float) (- (Variables|Default|GethygieneLevel) 2e+01) 0.0 1e+02))
  (Game|SpawnActorfromClass "/Game/Blueprints/Shit.Shit_C" (Math|Transform|MakeTransform (Math|Vector|MakeVector _x _y 7e+01) _rotation _scale) "Undefined" 0 0)
  (Variables|Default|SetshitNecessity 0.0)
  (Variables|Default|SetisNeedToShit false)
  (CallFunction|SetHumor)
  (CallFunction|FinishedTask "Coletar merda"))

(fn Eat
  (if (>= (Variables|Default|GethungryLevel) 1e+02)
    (Variables|Default|SetisHungry false)
    (Variables|Default|SetisEating false)
    (CallFunction|FinishedTask "Consertar alimentardor")
    (else
      (Utilities|Time|SetTimerbyFunctionName 0 "Eat" 2.0)
      (bind _output_get (Variables|Default|SethungryLevel (Math|Float|Clamp(Float) (+ (Variables|Default|GethungryLevel) 5.0) 0.0 1e+02)))
      (Development|PrintString (Utilities|String|Append "Hungry: " (Utilities|String|ToString(Float) _output_get)) true true "(R=1.000000,G=0.604231,B=0.000000,A=1.000000)" 4.8)))
  (CallFunction|SetHumor)
  (bind _output_get_2 (Variables|Default|SetshitNecessity (+ (Variables|Default|GetshitNecessity) 5.0)))
  (if (>= _output_get_2 8e+01)
    (Variables|Default|SetisNeedToShit true)))

(fn Sleep
  (Development|PrintString "tentei dormir")
  (if (>= (Variables|Default|GetsleepLevel) 1e+02)
    (Development|PrintString "sem sono")
    (Variables|Default|SetisSleeping false)
    (Variables|Default|SetisNeedToSleep false)
    (Variables|Default|SetisBusy false)
    (CallFunction|SetHumor)
    (CallFunction|FinishedTask)
    (else
      (if (Variables|Default|GetisSleeping)
        _
        (else
          (Variables|Default|SetisSleeping true)
          (AI|Navigation|StopMovement (Variables|Default|GetDinoController))
          (Development|PrintString "parei porra")))
      (Utilities|Time|SetTimerbyFunctionName 0 "Sleep" 2.0)
      (bind _output_get (Variables|Default|SetsleepLevel (Math|Float|Clamp(Float) (+ (Variables|Default|GetsleepLevel) 5.0) 0.0 1e+02)))
      (Variables|Default|SetisNeedToSleep (< _output_get 1e+01))
      (Development|PrintString (Utilities|String|Append "Sleep: " (Utilities|String|ToString(Float) _output_get)) true true "(R=1.000000,G=0.604231,B=0.000000,A=1.000000)" 4.8)
      (CallFunction|SetHumor))))

(fn Rage
  (Utilities|Time|SetTimerbyFunctionName 0 "Rage" 2.0)
  (bind _output_get (Variables|Default|SetfuryLevel (Math|Float|Clamp(Float) (- (Variables|Default|GetfuryLevel) 5.0) 0.0 1e+02)))
  (Development|PrintString (Utilities|String|Append "Fury: " (Utilities|String|ToString(Float) _output_get)) true true "(R=1.000000,G=0.604231,B=0.000000,A=1.000000)" 4.8))

(fn SetHumor
  (Default|SeekNewTask (Variables|Default|GetDinoController))
  (Development|PrintString "Humor")
  (bind _output_get (Variables|Default|Sethumor (/ (+ (Variables|Default|GethungryLevel) (Variables|Default|GethygieneLevel) (Variables|Default|GetsleepLevel)) 3.0)))
  (bind _asin_game (Utilities|Casting|CastToInGame (Game|GetGameMode)))
  (Default|UpdateHumor (Variables|/Game/Blueprints/Gameloop/InGame.InGame_C|GetHumorBar _asin_game) _output_get))

(fn Break
  (params (WallLife :type Float%20%28single-precision%29))
  (bind _damagecoeficient (Variables|Default|GetdamageCoeficient))
  (bind _returnvalue (- WallLife _damagecoeficient))
  (bind _returnvalue_2 (Math|Float|Clamp(Float) _returnvalue 0.0 1e+02))
  (Development|PrintString (Utilities|String|Append "golpe: " (Utilities|String|ToString(Float) _returnvalue_2)))
  (return _returnvalue_2))

(fn CooldowntoBreak
  (bind _breakcooldown (Variables|Default|GetbreakCooldown))
  (if (Variables|Default|GetisNeedToBreak)
    (Development|PrintString (Utilities|String|Append "cooldown Finished" (Utilities|String|ToString(Float) _breakcooldown)))
    (else
      (bind _result (Math|Float|IncrementFloat _breakcooldown)
        (:%20%20
          (Utilities|Time|SetTimerbyFunctionName 0 "CooldownToBreak" 1.0)
          (Variables|Default|SetisNeedToBreak (>= (Variables|Default|GetbreakCooldown) (Variables|Default|GetbreakCooldownBaseLevel)))
          (Development|PrintString (Utilities|String|ToString(Float) _result)))))))