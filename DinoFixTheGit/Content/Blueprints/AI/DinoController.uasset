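; AI controller for the Paper2D dino that acts on its needs and can smash walls to escape.
; SeekNewTask, when the dino is idle, prioritizes pooping, eating, sleeping and breaking walls, falling back to random patrol.
; Movement uses AIMoveTo toward tagged actors or the player, swapping flipbooks per action.
; A delayed loop damages the wall until the dino tires or breaks through, while Tick mirrors the sprite by Y velocity.
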(event Custom|GetNewPatrolPoint
  ;[1 1 1] Get Patrol Point of a single route
  (bind _outactors (Actor|GetAllActorswithTag "pr1"))
  (if (not (Variables|/Game/Blueprints/AI/PaperDino.PaperDino_C|GetisBusy (Variables|Default|GetPaperDino))) :!label _label
    (AI|AIMoveTo (Pawn|GetControlledPawn) "0, 0, 0" (Utilities|Array|Get(acopy) _outactors (Math|Random|RandomInteger (Utilities|Array|Length _outactors))) 5.0 false
      (:then
        (CallFunction|StartMoveAnim))
      (:OnSuccess
        (CallFunction|StopMoveAnim)
        (Utilities|FlowControl|Delay 2.0)
        (goto _label)))))

(event Custom|FollowPlayer
  ;[1 1 1] Follow the player
  (AI|AIMoveTo 0 "0, 0, 0" (Game|GetPlayerCharacter 0) 5.0 false
    (:then
      (CallFunction|StartMoveAnim))
    (:OnSuccess
      (CallFunction|StopMoveAnim))))

(event Custom|StopMoveAnim
  (Sprite|SetFlipbook (Variables|/Game/Blueprints/AI/PaperDino.PaperDino_C|GetPaperFlipbook (Variables|Default|GetPaperDino)) "/Game/Assets/Monster/Anim/Anim_Monster_Iddle.Anim_Monster_Iddle"))

(event Custom|GetWall
  (params (Wall :type Wall%20Corner%20Object%20Reference))
  ;[1 1 1] Break stuff
  (bind _output_get (Variables|Default|SetWall Wall)))

(event Custom|GoToFood
  (bind _paperdino (Variables|Default|GetPaperDino))
  (bind _paperdino_2 (Variables|Default|GetPaperDino))
  ;[1 1 1] Go to food
  (Variables|/Game/Blueprints/AI/PaperDino.PaperDino_C|SetisBusy _paperdino true)
  (bind _outactors (Actor|GetAllActorswithTag "food"))
  (AI|AIMoveTo _paperdino "0, 0, 0" (Utilities|Array|Get(acopy) _outactors) 2e+02 true
    (:then
      (CallFunction|StartMoveAnim))
    (:OnSuccess
      (CallFunction|StopMoveAnim)
      (Variables|/Game/Blueprints/AI/PaperDino.PaperDino_C|SetisHungry _paperdino_2 false)
      (Development|PrintString "Comendo")
      (Default|Eat _paperdino_2)
      (Variables|/Game/Blueprints/AI/PaperDino.PaperDino_C|SetisEating _paperdino_2 true)
      (Sprite|SetFlipbook (Variables|/Game/Blueprints/AI/PaperDino.PaperDino_C|GetPaperFlipbook (Variables|Default|GetPaperDino)) "/Game/Assets/Monster/Anim/Anim_Monster_Eat.Anim_Monster_Eat"))))

(event Custom|BreakStuff
  (bind _wall (Variables|Default|GetWall))
  (bind _paperdino (Variables|Default|GetPaperDino))
  ;[1 1 1] Break stuff
  (Variables|/Game/Blueprints/AI/PaperDino.PaperDino_C|SetisBusy (Variables|Default|GetPaperDino) true)
  (bind _outactors (Actor|GetAllActorswithTag "Wall"))
  (AI|AIMoveTo 0 "0, 0, 0" (Utilities|Array|Get(acopy) _outactors (Math|Random|RandomInteger (Utilities|Array|Length _outactors))) 5.0 true
    (:then
      (CallFunction|StartMoveAnim))
    (:OnSuccess
      (CallFunction|StopMoveAnim)
      (if (Actor|ActorHasTag "Wall")
        (Variables|Default|SetinitialWallLife (Variables|/Game/Blueprints/WallCorner.WallCorner_C|GetWallLife (stale Custom|GetWall _output_get)))
        ;;[1 1 1] "Break the wall" loop
        (bind _newwalllife (Default|Break (Variables|Default|GetPaperDino) (Variables|/Game/Blueprints/WallCorner.WallCorner_C|GetWallLife _wall) :!label _label))
        (Variables|/Game/Blueprints/WallCorner.WallCorner_C|SetWallLife _wall _newwalllife)
        (if (> _newwalllife 0.0)
          (if (<= _newwalllife (- 0.0 4e+01))
            (Utilities|FlowControl|Delay 2.0)
            (Development|PrintString "Cansei de quebrar")
            (Variables|/Game/Blueprints/AI/PaperDino.PaperDino_C|SetbreakCooldown _paperdino 0.0)
            (Variables|/Game/Blueprints/AI/PaperDino.PaperDino_C|SetisNeedToBreak _paperdino false)
            (Default|CooldowntoBreak _paperdino)
            (Variables|/Game/Blueprints/AI/PaperDino.PaperDino_C|SetisBusy _paperdino false)
            (Default|FinishedTask _paperdino "Consertar paredes!")
            (else
              (Utilities|FlowControl|Delay 2.0)
              (goto _label)))
          (else
            ;[1 1 1] Break the wall
            (Development|PrintString "parede quebrada")
            (Collision|SetCollisionEnabled (Variables|/Script/Engine.StaticMeshActor|GetStaticMeshComponent _wall) "NoCollision")
            ;[1 1 1] Try to escape when a wall breaks
            (Utilities|FlowControl|Delay 2.0)
            (CallFunction|TrytoEscape)))))))

(event Custom|TryToEscape
  ;[1 1 1] Escape!
  (Variables|/Game/Blueprints/AI/PaperDino.PaperDino_C|SetisBusy (Variables|Default|GetPaperDino) true)
  (bind _outactors (Actor|GetAllActorswithTag "escape"))
  (AI|AIMoveTo (Variables|Default|GetPaperDino) "0, 0, 0" (Utilities|Array|Get(acopy) _outactors) 1.0 true
    (:then
      (CallFunction|StartMoveAnim))
    (:OnSuccess
      (CallFunction|StopMoveAnim))))

(event Custom|TryToShit
  (bind _paperdino (Variables|Default|GetPaperDino))
  ;[1 1 1] Make shit
  (Variables|/Game/Blueprints/AI/PaperDino.PaperDino_C|SetisBusy _paperdino true)
  (Utilities|FlowControl|Delay 2.0)
  (Default|Shit _paperdino)
  (Sprite|SetFlipbook (Variables|/Game/Blueprints/AI/PaperDino.PaperDino_C|GetPaperFlipbook (Variables|Default|GetPaperDino)) "/Game/Assets/Monster/Anim/Anim_Monster_Pooping.Anim_Monster_Pooping"))

(event Custom|TryToSleep
  (bind _paperdino (Variables|Default|GetPaperDino))
  (Sprite|SetFlipbook (Variables|/Game/Blueprints/AI/PaperDino.PaperDino_C|GetPaperFlipbook (Variables|Default|GetPaperDino)) "/Game/Assets/Monster/Anim/Anim_Monster_Sleep.Anim_Monster_Sleep")
  ;[1 1 1] Fall to sleep
  (Variables|/Game/Blueprints/AI/PaperDino.PaperDino_C|SetisBusy _paperdino true)
  (Utilities|FlowControl|Delay 2.0)
  (Default|Sleep _paperdino)
  (Sprite|SetFlipbook (Variables|/Game/Blueprints/AI/PaperDino.PaperDino_C|GetPaperFlipbook (Variables|Default|GetPaperDino)) "/Game/Assets/Monster/Anim/Anim_Monster_Sleep.Anim_Monster_Sleep"))

(event Custom|SeekNewTask
  (bind _paperdino (Variables|Default|GetPaperDino))
  ;[1 1 1] Look for a new task
  (if (not (Variables|/Game/Blueprints/AI/PaperDino.PaperDino_C|GetisBusy _paperdino))
    (if (Variables|/Game/Blueprints/AI/PaperDino.PaperDino_C|GetisNeedToShit _paperdino)
      (CallFunction|TrytoShit)
      (elif (Variables|/Game/Blueprints/AI/PaperDino.PaperDino_C|GetisHungry _paperdino)
        (CallFunction|GotoFood)
        (elif (Variables|/Game/Blueprints/AI/PaperDino.PaperDino_C|GetisNeedToSleep _paperdino)
          (CallFunction|TrytoSleep)
          (elif (Variables|/Game/Blueprints/AI/PaperDino.PaperDino_C|GetisNeedToBreak _paperdino)
            (CallFunction|BreakStuff)
            (else
              (CallFunction|GetNewPatrolPoint))))))))

(event Custom|StartMoveAnim
  (Sprite|SetFlipbook (Variables|/Game/Blueprints/AI/PaperDino.PaperDino_C|GetPaperFlipbook (Variables|Default|GetPaperDino)) "/Game/Assets/Monster/Anim/Anim_Monster_Run.Anim_Monster_Run"))

(event EventBeginPlay
  ;[1 1 1] Start and set Paper Dino
  (bind _aspaper_dino (Utilities|Casting|CastToPaperDino (Pawn|GetControlledPawn)))
  (Variables|Default|SetPaperDino _aspaper_dino))

(event EventTick
  (params (DeltaSeconds :type Float%20%28single-precision%29))
  (bind _paperdino (Variables|Default|GetPaperDino))
  (bind _paperflipbook (Variables|/Game/Blueprints/AI/PaperDino.PaperDino_C|GetPaperFlipbook _paperdino))
  ;[1 1 1] Flipa
  (Math|Float|CompareFloat (.y (Variables|/Script/Engine.MovementComponent|GetVelocity (Variables|/Script/Engine.Character|GetCharacterMovement _paperdino))) 0.0
    (:>
      (Transformation|SetWorldScale3D _paperflipbook (Math|Vector|MakeVector -0.8 0.8 0.8)))
    (:<
      (Transformation|SetWorldScale3D _paperflipbook (Math|Vector|MakeVector 0.8 0.8 0.8)))))

(fn ConstructionScript)